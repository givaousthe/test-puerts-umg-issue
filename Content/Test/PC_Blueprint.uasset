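; Test Blueprint, apparently a player controller, for watching how UObject counts respond to UMG widget creation, removal and garbage collection.
; Z creates a BlueprintUMG widget and adds it to the viewport, X removes the most recently created one, and C calls garbage collection.
; Every Tick prints object array statistics on screen without logging, including total, available and permanent counts, to show when objects are freed.
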(event Custom|PrintUobjectNumber
  (params (PrintToLog :type Boolean))
  (Development|PrintString (Utilities|String|Append "num: " (Utilities|String|ToString(Integer) (Class|TestUMG|GetObjectArrayNum)) " 
num minus available: " (Utilities|String|ToString(Integer) (Class|TestUMG|GetObjectArrayNumMinusAvailable)) " 
num minus permanent: " (Utilities|String|ToString(Integer) (Class|TestUMG|GetObjectArrayNumMinusPermanent)) " 
num permanent: " (Utilities|String|ToString(Integer) (Class|TestUMG|GetObjectArrayNumPermanent)) " 
num estimated available: " (Utilities|String|ToString(Integer) (Class|TestUMG|GetObjectArrayEstimatedAvailable))) true PrintToLog "(R=0.000000,G=1.000000,B=0.058869,A=1.000000)" 0.0))

(event EventBeginPlay)

(event EventTick
  (params (DeltaSeconds :type Float%20%28single-precision%29))
  (CallFunction|PrintUobjectNumber false))

(event Input|KeyboardEvents|Z
  (params (Key :type Key%20Structure :default "None"))
  (:Pressed
    (bind _returnvalue (UserInterface|CreateWidget "/Game/Test/BlueprintUMG.BlueprintUMG_C"))
    (UserInterface|Viewport|AddtoViewport _returnvalue 0)))

(event Input|KeyboardEvents|C
  (params (Key :type Key%20Structure :default "None"))
  (:Pressed
    (Utilities|Platform|CollectGarbage)))

(event Input|KeyboardEvents|X
  (params (Key :type Key%20Structure :default "None"))
  (:Pressed
    (Widget|RemovefromParent (stale Input|KeyboardEvents|Z _returnvalue))))

(fn ConstructionScript)